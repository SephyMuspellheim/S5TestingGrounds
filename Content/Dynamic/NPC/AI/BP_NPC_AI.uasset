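; BP_NPC_AI is an AI controller for guard NPCs that detects targets through AI Perception.
; On BeginPlay it initializes the BB_PatrolData blackboard and runs the BT_GuardBehaviour behavior tree.
; Perception updates ignore actors tagged "Enemy"; any other sensed actor is written to the Enemy blackboard key, which is cleared when sensing of such an actor fails.
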(event `self.ReceiveBeginPlay`
  (bind _blackboardcomponent (`self.UseBlackboard` "/Game/Dynamic/NPC/AI/BB_PatrolData.BB_PatrolData"))
  (`self.RunBehaviorTree` "/Game/Dynamic/NPC/AI/BT_GuardBehaviour.BT_GuardBehaviour")
  (set `self.BlackboardComp` _blackboardcomponent))

(event `self.AIPerception.OnTargetPerceptionUpdated`
  (params (Actor :type "Actor Object Reference") (Stimulus :type "AIStimulus Structure"))
  (bind _blackboardcomp (`self.BlackboardComp`))
  (bind _enemy (`self.Enemy`))
  (if (`self.ActorHasTag` Actor "Enemy")
    _
    (elif (`.bSuccessfullySensed` (break `AIStimulus` Stimulus))
      (`BlackboardComponent.SetValueAsObject` _blackboardcomp _enemy Actor)
      (else
        (`BlackboardComponent.ClearValue` _blackboardcomp _enemy)))))

(fn `UserConstructionScript`)