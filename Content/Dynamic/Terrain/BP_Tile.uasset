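; BP_Tile is one segment of an infinite terrain, scattering props, rocks and AI pawns on BeginPlay.
; Its barrier starts locked, unlocks while the player overlaps the locking volume, then relocks on exit to prevent backtracking and reports completion to the game mode once.
; Player overlap with the destroy volume asks the game mode to spawn another tile and destroys this one.
; An arrow component supplies the attach transform for chaining tiles.
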(event `self.ReceiveBeginPlay`
  ;[1 1 1] Set tiles to locked to prevent backtracking
  (`self.Lock`)
  (`self.PlaceActors` "/Game/Dynamic/Terrain/Props/BP_Container.BP_Container_C" 1 3 400.0)
  (`self.PlaceActors` "/Game/Dynamic/Terrain/Props/BP_SandBags.BP_SandBags_C" 1 3 200.0)
  (`self.PlaceActors` "/Game/Dynamic/Terrain/Props/BP_Box.BP_Box_C" 1 3 250.0 1.0 3.0)
  (`self.PlaceActors` "/Game/Dynamic/Terrain/Props/BP_Rock1.BP_Rock1_C" 1 3 500.0 0.5 5.0)
  (`self.PlaceActors` "/Game/Dynamic/Terrain/Props/BP_Rock5.BP_Rock5_C" 1 3 400.0 0.5 2.0)
  (`self.PlaceActors` "/Game/Dynamic/Terrain/Props/BP_Rock7.BP_Rock7_C" 1 3 450.0 0.5 2.0)
  (`self.PlaceAIPawns` "/Game/Dynamic/Character/Behaviour/BP_Character.BP_Character_C" 2 5 100.0))

(event `self.LockingVolume.OnComponentBeginOverlap`
  (params (OverlappedComponent :type "PrimitiveComponent Object Reference") (OtherActor :type "Actor Object Reference") (OtherComp :type "PrimitiveComponent Object Reference") (OtherBodyIndex :type Integer) (bFromSweep :type Boolean) (SweepResult :type "HitResult Structure (by ref)"))
  ;[1 1 1] When player enters tile, unlock end gate
  (`self.IsPlayerActor?` OtherActor)
  (`self.Unlock`))

(event `self.LockingVolume.OnComponentEndOverlap`
  (params (OverlappedComponent :type "PrimitiveComponent Object Reference") (OtherActor :type "Actor Object Reference") (OtherComp :type "PrimitiveComponent Object Reference") (OtherBodyIndex :type Integer))
  ;[1 1 1] When player leaves tile, close previous gate || When player enters destroy volume, destroy referenced tile (Prev+1)
  (`self.IsPlayerActor?` OtherActor)
  (`self.Lock`)
  (`self.TileComplete`))

(event `self.DestroyVolume.OnComponentBeginOverlap`
  (params (OverlappedComponent :type "PrimitiveComponent Object Reference") (OtherActor :type "Actor Object Reference") (OtherComp :type "PrimitiveComponent Object Reference") (OtherBodyIndex :type Integer) (bFromSweep :type Boolean) (SweepResult :type "HitResult Structure (by ref)"))
  ;[1 1 1] When player leaves tile, close previous gate || When player enters destroy volume, destroy referenced tile (Prev+1)
  (`self.IsPlayerActor?` OtherActor)
  (bind _asbp_infinite_terrain_game_mode (cast `/Game/Dynamic/BP_InfiniteTerrainGameMode` (`GameplayStatics.GetGameMode`)))
  (`/Game/Dynamic/BP_InfiniteTerrainGameMode.Spawn Tile` _asbp_infinite_terrain_game_mode)
  (`self.K2_DestroyActor`))

(fn `GetAttachLocation`
  (returns (AttachTransform :type "Transform Structure"))
  (return (`SceneComponent.K2_GetComponentToWorld` (`self.Arrow`))))

(fn `Lock`
  (bind _barrier (`self.Barrier`))
  (`PrimitiveComponent.SetCollisionEnabled` _barrier "QueryAndPhysics")
  (`PrimitiveComponent.SetMaterial` _barrier 0 "/Game/Dynamic/Terrain/MI_Barrier_Locked.MI_Barrier_Locked"))

(fn `SpawnTile`
  (params (Amount :type Integer))
  (returns (Tiles :type "Array of /Game/Dynamic/Terrain/BP_Tile Object Reference"))
  (for _ (range 1 (+ Amount 1))
    (bind _returnvalue (`|SpawnActorFromClass` "BP_Tile_C" (`self.NextTileTransform`) "Undefined" "OverrideRootScale" null null))
    (`KismetArrayLibrary.Array_Add` (`self.Tiles`) _returnvalue)
    (bind _attachtransform (`self.GetAttachLocation` _returnvalue))
    (set `self.NextTileTransform` _attachtransform))
  (return (`self.Tiles`)))

(fn `TileComplete`
  (if (not (`self.isTileComplete`))
    (bind _asbp_infinite_terrain_game_mode (cast `/Game/Dynamic/BP_InfiniteTerrainGameMode` (`GameplayStatics.GetGameMode`)))
    (`/Game/Dynamic/BP_InfiniteTerrainGameMode.TileComplete` _asbp_infinite_terrain_game_mode)
    (set `self.isTileComplete` true)))

(fn `Unlock`
  (bind _barrier (`self.Barrier`))
  (`PrimitiveComponent.SetCollisionEnabled` _barrier "NoCollision")
  (`PrimitiveComponent.SetMaterial` _barrier 0 "/Game/Dynamic/Terrain/MI_Barrier_Unlocked.MI_Barrier_Unlocked"))

(fn `UserConstructionScript`)